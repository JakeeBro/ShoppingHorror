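; BP_ListManager is a debug actor that prints the contents of a class-keyed map to the screen.
; Shortly after BeginPlay it calls WriteListClass, converts the result with MapListToStrings, and prints each resulting key.
; An unconnected branch would print every entry's index, class name and value, using SplitClassName to strip the BP_ prefix and _C suffix.
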(event EventBeginPlay
  (Utilities|FlowControl|Delay 0.5)
  (bind _returnvalue (Class|ListManager|WriteListClass))
  (bind _returnvalue_2 (Class|ListManager|MapListtoStrings _returnvalue))
  (bind _keys (Utilities|Map|Keys _returnvalue_2))
  (for _array_element _keys
    (Development|PrintString _array_element true false "(R=1.000000,G=0.724435,B=0.264536,A=1.000000)" 2e+01)))

(event Collision|EventActorBeginOverlap
  (params (OtherActor :type Actor%20Object%20Reference)))

(event EventTick
  (params (DeltaSeconds :type Float%20%28single-precision%29)))

(fn ConstructionScript)

(fn SplitClassName
  (params (Class%20Display%20Name :type String))
  (return (.LeftS (Utilities|String|Split (.RightS (Utilities|String|Split Class%20Display%20Name "BP_")) "_C"))))