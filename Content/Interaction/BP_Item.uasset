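; BP_Item is an interactable pickup item that moves itself into the interacting player's inventory.
; On Interact it gets the Player from the interacting actor, passes itself and its ItemProperties to that player's inventory via AddToInventory, then destroys itself.
; Several disconnected node chains hold unused alternatives, including held-list tracking with per-item counts and debug prints.
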(event EventBeginPlay)

(event Collision|EventActorBeginOverlap
  (params (OtherActor :type Actor%20Object%20Reference)))

(event EventTick
  (params (DeltaSeconds :type Float%20%28single-precision%29)))

(event EventInteract
  (params (Actor :type Actor%20Object%20Reference))
  (bind _self self)
  (bind _returnvalue (Class|PlayerInterface|GetPlayer(Message) Actor))
  (Variables|Default|SetPlayer _returnvalue)
  (Utilities|FlowControl|Sequence
    (:then_0
      (bind _returnvalue_2 (Class|PlayerInterface|GetInventory(Message) (Variables|Default|GetPlayer)))
      (Class|Inventory|AddtoInventory _returnvalue_2 _self (Variables|Default|GetItemProperties _self))
      (Actor|DestroyActor))))

(fn ConstructionScript)